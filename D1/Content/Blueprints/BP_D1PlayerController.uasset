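; BP_D1PlayerController is a player controller that shows a player score HUD and can switch which pawn the player controls.
; On BeginPlay it creates a WBP_PlayerScore widget, stores the reference and adds it to the viewport.
; ChangePlayer releases the current pawn, then possesses the Players entry at the given index, so an invalid index leaves the controller without a pawn.
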(event `self.ReceiveBeginPlay`
  (bind _returnvalue (`|CreateWidget` "/Game/UI/WBP_PlayerScore.WBP_PlayerScore_C" self))
  (bind _output_get (set `self.PlayerScoreWidget` _returnvalue))
  (`UserWidget.AddToViewport` _output_get 0))

(fn `ChangePlayer`
  (params (Index :type Integer))
  (`self.UnPossess`)
  (if (`KismetArrayLibrary.Array_IsValidIndex` (`self.Players`) Index)
    (`self.Possess` (`|GetArrayItem` (`self.Players`) (`local.Index`)))))

(fn `UserConstructionScript`)